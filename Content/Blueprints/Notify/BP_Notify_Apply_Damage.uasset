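; Animation notify state that marks the window in an attack animation during which the owner's primary weapon is attacking.
; Begin and End fetch the weapon from the mesh owner through GetPrimaryWeaponMessage, then start the attack, or stop and reset it, if valid.
; Tick makes the same query on the mesh's attach parent but does nothing with the result.
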(fn ReceivedNotifyTick
  (params (MeshComp :type Skeletal%20Mesh%20Component%20Object%20Reference) (Animation :type Anim%20Sequence%20Base%20Object%20Reference) (FrameDeltaTime :type Float%20%28single-precision%29))
  (Class|BICharacterInformation|GetPrimaryWeapon(Message) (Transformation|GetAttachParent MeshComp)))

(fn ReceivedNotifyBegin
  (params (MeshComp :type Skeletal%20Mesh%20Component%20Object%20Reference) (Animation :type Anim%20Sequence%20Base%20Object%20Reference) (TotalDuration :type Float%20%28single-precision%29))
  (bind _actor (Class|BICharacterInformation|GetPrimaryWeapon(Message) (Components|GetOwner MeshComp)))
  (Utilities|IsValid _actor
    (:Is%20Valid
      (Default|StartAttack _actor)
      (return false))))

(fn ReceivedNotifyEnd
  (params (MeshComp :type Skeletal%20Mesh%20Component%20Object%20Reference) (Animation :type Anim%20Sequence%20Base%20Object%20Reference))
  (bind _actor (Class|BICharacterInformation|GetPrimaryWeapon(Message) (Components|GetOwner MeshComp)))
  (Utilities|IsValid _actor
    (:Is%20Valid
      (Default|StopAttack _actor)
      (Default|ResetAttack _actor)
      (return false))))