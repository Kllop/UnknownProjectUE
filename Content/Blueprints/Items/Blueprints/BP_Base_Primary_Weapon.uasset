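; Base primary weapon Blueprint that deals fixed point damage through a melee-style swept trace.
; StartAttack and StopAttack control the CheckAttack timeline, whose update is meant to run a sphere trace from the arrow along the capsule's length.
; An ignore list limits damage to once per actor until ResetAttack clears it.
; A separate capsule hit handler prints a debug message and calls point damage without a target connected.
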(event OnComponentHit(Capsule1)
  (params (HitComponent :type Primitive%20Component%20Object%20Reference) (OtherActor :type Actor%20Object%20Reference) (OtherComp :type Primitive%20Component%20Object%20Reference) (NormalImpulse :type Vector :default "0, 0, 0") (Hit :type Hit%20Result%20Structure%20%28by%20ref%29))
  (bind _returnvalue (Components|GetOwner))
  (if (!= OtherActor _returnvalue)
    (Game|Damage|ApplyPointDamage 0 1e+01 (.Location (Collision|BreakHitResult Hit)) Hit (Game|GetInstigatorController _returnvalue) _returnvalue "/Game/Blueprints/DamageType/TEST_DamageType.TEST_DamageType_C")
    (Development|PrintString "Hello")))

(event EventTick
  (params (DeltaSeconds :type Float%20%28single-precision%29)))

(fn ConstructionScript
  (|CallParentFunction))

(fn DrawCapsuleTrace
  (bind _returnvalue (Components|GetOwner))
  (bind _arrow (Variables|Default|GetArrow))
  (bind _returnvalue_2 (Transformation|GetWorldLocation _arrow))
  (bind (_outhit _returnvalue_3) (Collision|SphereTraceByChannel _returnvalue_2 (+ _returnvalue_2 (* (Math|Vector|GetForwardVector (Transformation|GetWorldRotation _arrow)) (* (Variables|/Script/Engine.CapsuleComponent|GetCapsuleHalfHeight (Variables|Default|GetCapsule1)) 2.0))) (+ (Variables|/Script/Engine.CapsuleComponent|GetCapsuleRadius (Variables|Default|GetCapsule1)) 5.0) "TraceTypeQuery2" false (Utilities|Array|MakeArray (Components|GetOwner)) "None"))
  (if _returnvalue_3
    (if (== (Utilities|Array|FindItem (Variables|Default|GetActorsIgnore) (.HitActor (Collision|BreakHitResult _outhit))) -1)
      (Game|Damage|ApplyPointDamage (.HitActor (Collision|BreakHitResult _outhit)) 1e+01 (.Location (Collision|BreakHitResult _outhit)) _outhit (Game|GetInstigatorController _returnvalue) _returnvalue)
      (Utilities|Array|Add (Variables|Default|GetActorsIgnore) (.HitActor (Collision|BreakHitResult _outhit)))
      (return))))

(fn StartAttack
  (Components|Timeline|PlayfromStart (Variables|Default|GetCheckAttack)))

(fn StopAttack
  (Audio|Components|Audio|Stop (Variables|Default|GetCheckAttack)))

(fn ResetAttack
  (Utilities|Array|Clear (Variables|Default|GetActorsIgnore)))