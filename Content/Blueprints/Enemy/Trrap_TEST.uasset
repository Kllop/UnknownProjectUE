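; Test trap actor that spins continuously around yaw and damages actors overlapping either of its two box colliders.
; On overlap, each box runs a stationary, enlarged box trace for Pawns with debug drawing, whose success gates point damage to the overlapping actor.
; Each box has its own DoOnce and one-second reset timer, acting as a hit cooldown.
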(event OnComponentBeginOverlap(Box)
  (params (OverlappedComponent :type Primitive%20Component%20Object%20Reference) (OtherActor :type Actor%20Object%20Reference) (OtherComp :type Primitive%20Component%20Object%20Reference) (OtherBodyIndex :type Integer) (bFromSweep :type Boolean) (SweepResult :type Hit%20Result%20Structure%20%28by%20ref%29))
  (bind _box (Variables|Default|GetBox))
  (bind _returnvalue (Transformation|GetWorldLocation _box))
  (bind (_outhit _returnvalue_2) (Class|KismetSystemLibrary|BoxTraceSingleforObjects _returnvalue _returnvalue (* (Variables|/Script/Engine.BoxComponent|GetBoxExtent _box) 2.3) (Transformation|GetWorldRotation _box) (Utilities|Array|MakeArray "ObjectTypeQuery3") false 0 "ForDuration" true "(R=1.000000,G=0.000000,B=0.000000,A=1.000000)" "(R=0.000000,G=1.000000,B=0.000000,A=1.000000)" 1.0))
  (if _returnvalue_2
    (Utilities|FlowControl|DoOnce false
      (:Completed
        (Game|Damage|ApplyPointDamage OtherActor 5.0 (.Location (Collision|BreakHitResult _outhit)) _outhit 0 self "/Game/Blueprints/DamageType/TEST_DamageType.TEST_DamageType_C")
        (Utilities|Time|SetTimerbyEvent (EventDispatchers|CreateEvent :!event Custom|Reset_01) 1.0)))))

(event OnComponentBeginOverlap(Box1)
  (params (OverlappedComponent :type Primitive%20Component%20Object%20Reference) (OtherActor :type Actor%20Object%20Reference) (OtherComp :type Primitive%20Component%20Object%20Reference) (OtherBodyIndex :type Integer) (bFromSweep :type Boolean) (SweepResult :type Hit%20Result%20Structure%20%28by%20ref%29))
  (bind _box1 (Variables|Default|GetBox1))
  (bind _returnvalue (Transformation|GetWorldLocation _box1))
  (bind (_outhit _returnvalue_2) (Class|KismetSystemLibrary|BoxTraceSingleforObjects _returnvalue _returnvalue (* (Variables|/Script/Engine.BoxComponent|GetBoxExtent _box1) 2.3) (Transformation|GetWorldRotation _box1) (Utilities|Array|MakeArray "ObjectTypeQuery3") false 0 "ForDuration" true "(R=1.000000,G=0.000000,B=0.000000,A=1.000000)" "(R=0.000000,G=1.000000,B=0.000000,A=1.000000)" 1.0))
  (if _returnvalue_2
    (Utilities|FlowControl|DoOnce false
      (:Completed
        (Game|Damage|ApplyPointDamage OtherActor 5.0 (.Location (Collision|BreakHitResult _outhit)) _outhit 0 self "/Game/Blueprints/DamageType/TEST_DamageType.TEST_DamageType_C")
        (Utilities|Time|SetTimerbyEvent (EventDispatchers|CreateEvent :!event Custom|Reset_02) 1.0)))))

(event Custom|Reset_01
  (Utilities|FlowControl|DoOnce false) ; enters at Reset
)

(event Custom|Reset_02
  (Utilities|FlowControl|DoOnce false) ; enters at Reset
)

(event EventTick
  (params (DeltaSeconds :type Float%20%28single-precision%29))
  (Transformation|AddRelativeRotation (Variables|Default|GetScene) (Math|Rotator|MakeRotator 0.0 0.0 (* DeltaSeconds 5e+01)) false false))

(fn ConstructionScript)